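; Arcane Shards ability that shows a magic circle, then on input press bursts a series of shards around the targeted ground point.
; A spawned point collection supplies randomly rotated ground points, their count set by ability level up to a cap.
; After the cast montage event, cost commits and a looping timer fires each shard's cue and radial damage with outward knockback.
; When all shards finish, it commits cooldown and ends.
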(event Custom|SpawnShard
  (if (< (Variables|Default|GetCount) (Variables|Default|GetNum%20Shards))
    (CallFunction|StoreShardSpawnLocation)
    (CallFunction|StorePlayerstoDamage)
    (for _array_element (Variables|Default|GetPlayersToDamage)
      (CallFunction|RadialDamagetoPlayer _array_element))
    (Math|Integer|IncrementInt (Variables|Default|GetCount)
      (:%20%20
        (Class|GameplayAbility|ExecuteGameplayCuewithParams "(TagName=\"GameplayCue.ArcaneShards\")" (Ability|GameplayCue|MakeGameplayCueParameters :Location (Variables|Default|GetShardSpawnLocation)))))
    (else
      (Utilities|Time|ClearandInvalidateTimerbyHandle (Variables|Default|GetShardSpawnTimer))
      (Actor|DestroyActor (Variables|Default|GetPoint%20Collection))
      (Ability|CommitAbilityCooldown false)
      (Ability|EndAbility))))

(event Ability|EventActivateAbility
  (bind _returnvalue (Class|GameplayAbility|CheckAbilityCost))
  (if _returnvalue
    (Utilities|FlowControl|Sequence
      (:then_0
        (Class|PlayerInterface|ShowMagicCircle(Message) (Ability|GetAvatarActorfromActorInfo) 0))
      (:then_1
        (Ability|Tasks|WaitInputPress false
          (:OnPress
            (bind _datahandle (|TargetDataUnderMouse)
              (:ValidData
                (bind _output_get (Variables|Default|SetMouseHitLocation (.ImpactPoint (Collision|BreakHitResult (Ability|TargetData|GetHitResultfromTargetData _datahandle)))))
                (bind _returnvalue_2 (Game|SpawnActorfromClass "/Game/Blueprints/AbilitySystem/Aura/Abilities/Arcane/ArcaneShards/BP_PointCollection.BP_PointCollection_C" (Math|Transform|MakeTransform _output_get "0, 0, 0" "1.000000,1.000000,1.000000") "AlwaysSpawn" "MultiplyWithRoot" 0 0))
                (Variables|Default|SetPoint%20Collection _returnvalue_2)
                (Variables|Default|SetNum%20Shards (Math|Integer|Min(Integer) (Variables|Default|GetMaxNumShards) (Ability|GetAbilityLevel)))
                (Variables|Default|SetGroundPoints (Class|PointCollection|GetGroundPoints (Variables|Default|GetPoint%20Collection) (Variables|Default|GetMouseHitLocation) (Variables|Default|GetNum%20Shards) (Math|Random|RandomFloatinRange 0.0 3.6e+02)))
                (Class|CombatInterface|UpdateFacingTarget(Message) (Ability|GetAvatarActorfromActorInfo) (Variables|Default|GetMouseHitLocation))
                (|PlayMontageandWaitProxy "None" "/Game/Assets/Characters/Aura/Animations/Abilities/AM_Cast_ArcaneShards.AM_Cast_ArcaneShards" 1.0 "None" false 1.0 0.0 false
                  (:then
                    (Ability|Tasks|WaitGameplayEvent "(TagName=\"Event.Montage.ArcaneShards\")" 0
                      (:EventReceived
                        (bind _returnvalue_3 (Utilities|Time|SetTimerbyEvent (delegate Custom|SpawnShard) (Variables|Default|GetShardSpawnDeltaTime) true))
                        (Variables|Default|SetShardSpawnTimer _returnvalue_3)
                        (Class|PlayerInterface|HideMagicCircle(Message) (Ability|GetAvatarActorfromActorInfo))
                        (CallFunction|SpawnShard)
                        (Ability|CommitAbilityCost false)))))))))))))

(event Ability|EventOnEndAbility
  (params (bWasCancelled :type Boolean)))

(fn StoreShardSpawnLocation
  (Variables|Default|SetShardSpawnLocation (Transformation|GetWorldLocation (Utilities|Array|Get(acopy) (Variables|Default|GetGroundPoints) (Variables|Default|GetCount)))))

(fn StorePlayerstoDamage
  (bind _returnvalue (Ability|GetAvatarActorfromActorInfo))
  (bind _outoverlappingactors (Class|AuraAbilitySystemLibrary|GetLivePlayersWithinRadius _returnvalue (Utilities|Array|MakeArray _returnvalue) (Variables|Default|GetRadialDamageOuterRadius) (Variables|Default|GetShardSpawnLocation)))
  (Variables|Default|SetPlayersToDamage _outoverlappingactors))

(fn RadialDamagetoPlayer
  (params (TargetActor :type Actor%20Object%20Reference))
  (bind _returnvalue (Transformation|GetActorLocation TargetActor))
  (bind _shardspawnlocation (Variables|Default|GetShardSpawnLocation))
  (bind _returnvalue_2 (- _returnvalue _shardspawnlocation))
  (Class|AuraAbilitySystemLibrary|ApplyDamageEffect (Class|AuraDamageGameplayAbility|MakeDamageEffectParamsfromClassDefaults TargetActor _shardspawnlocation true _returnvalue_2 true _returnvalue_2 true 35.0)))